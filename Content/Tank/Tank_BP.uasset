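; Player-controllable tank Blueprint that maps input to camera orbit, driving and firing.
; On BeginPlay it hands the barrel and turret to the TankAiming component and both tracks to TankMovement.
; Aim axes rotate an azimuth gimbal for yaw and the spring arm for pitch separately, scaled by delta time.
; Movement axes pass intents to TankMovement, and the Fire action calls TankAiming.
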(event EventBeginPlay
  (Class|TankAimingComponent|Initialize (Variables|Default|GetTank%20Aiming) (Variables|Default|GetTank%20Barrel) (Variables|Default|GetTank%20Turret))
  (Class|TankMovementComponent|Initialize (Variables|Default|GetTank%20Movement) (Variables|Default|GetLeftTrack) (Variables|Default|GetRightTrack)))

(event Input|ActionEvents|InputActionFire
  (params (Key :type Key%20Structure))
  (:Pressed
    (Class|TankAimingComponent|Fire (Variables|Default|GetTank%20Aiming))))

(event Input|AxisEvents|InputAxisAimAzimuth
  (params (AxisValue :type Float%20%28single-precision%29))
  ;[1 1 1] Camera Input Binding
  (Transformation|AddLocalRotation (Variables|Default|GetAzimuthGimbalScene) (Math|Rotator|MakeRotator 0.0 0.0 (* AxisValue (Utilities|Time|GetWorldDeltaSeconds) 1e+02)) false false))

(event Input|AxisEvents|InputAxisAimElevation
  (params (AxisValue :type Float%20%28single-precision%29))
  ;[1 1 1] Camera Input Binding
  (Transformation|AddLocalRotation (Variables|Default|GetSpringArm) (Math|Rotator|MakeRotator 0.0 (* AxisValue (Utilities|Time|GetWorldDeltaSeconds) 1e+02) 0.0) false false))

(event Input|AxisEvents|InputAxisForward
  (params (AxisValue :type Float%20%28single-precision%29))
  ;[1 1 1] Movement
  (Class|TankMovementComponent|IntendMoveForward (Variables|Default|GetTank%20Movement) AxisValue))

(event Input|AxisEvents|InputAxisTurnRight
  (params (AxisValue :type Float%20%28single-precision%29))
  ;[1 1 1] Movement
  (Class|TankMovementComponent|IntendMoveRight (Variables|Default|GetTank%20Movement) AxisValue))

(fn ConstructionScript)